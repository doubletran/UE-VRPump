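; GrabbableTool is a grabbable component that gives its parent static mesh highlight feedback.
; On BeginPlay it caches that mesh, enables overlap events and binds the grab, drop and highlight events.
; Highlighting toggles the material's Speed parameter, creating a dynamic material instance on each change.
; Grabbing saves the parent's world transform in OldLocation, which is not read here, and the drop handler is empty.
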(event `OnHighlighted_Event`
  (bind _mesh (`self.Mesh`))
  (bind _returnvalue (`PrimitiveComponent.CreateDynamicMaterialInstance` _mesh 0 (`PrimitiveComponent.GetMaterial` _mesh 0) "None"))
  (`MaterialInstanceDynamic.SetScalarParameterValue` _returnvalue "Speed" 1.0))

(event `StopHighlight`
  (bind _mesh (`self.Mesh`))
  (bind _returnvalue (`PrimitiveComponent.CreateDynamicMaterialInstance` _mesh 0 (`PrimitiveComponent.GetMaterial` _mesh 0) "None"))
  (`MaterialInstanceDynamic.SetScalarParameterValue` _returnvalue "Speed" 0.0))

(event `self.ReceiveBeginPlay`
  (`parent.ReceiveBeginPlay`)
  (bind _asstatic_mesh_component (cast `StaticMeshComponent` (`self.GetAttachParent`)))
  (set `PrimitiveComponent.bGenerateOverlapEvents` true _asstatic_mesh_component)
  (set `self.Mesh` _asstatic_mesh_component)
  (add `self.OnDropped` (delegate `OnDropped_Event`))
  (add `self.OnHighlight` (delegate `OnHighlighted_Event`))
  (add `self.OnStopHighlight` (delegate `StopHighlight`))
  (add `self.OnGrabbed` (delegate `OnGrabbed_Event`)))

(event `OnGrabbed_Event`
  (set `self.OldLocation` (`self.K2_GetComponentToWorld` (`self.GetAttachParent`))))

(event `OnDropped_Event`)

(fn `NewFunction_0`)