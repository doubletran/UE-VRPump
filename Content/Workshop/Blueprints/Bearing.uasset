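; Bearing is a workshop part actor that reacts to being dropped and can spin its inner race through a Rotate function.
; Mesh hits check actor tags, broadcasting a table landing and then clearing its listeners, or a ground landing with a metal drop sound.
; Shaft overlaps only print debug text, and the handler bound to the GrabbableTool drop event is empty.
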(event `self.ReceiveBeginPlay`
  (bind _returnvalue (`self.GetComponentByClass` "/Game/Workshop/Blueprints/GrabbableTool.GrabbableTool_C"))
  (`/Engine/EditorBlueprintResources/StandardMacros.IsValid` _returnvalue
    (:`Is Valid`
      (add `/Game/VRTemplate/Blueprints/GrabComponent.OnDropped` _returnvalue (delegate `OnDropped`)))))

(event `OnDropped`)

(event `self.StaticMeshComponent.OnComponentBeginOverlap`
  (params (OverlappedComponent :type "PrimitiveComponent Object Reference") (OtherActor :type "Actor Object Reference") (OtherComp :type "PrimitiveComponent Object Reference") (OtherBodyIndex :type Integer) (bFromSweep :type Boolean) (SweepResult :type "HitResult Structure (by ref)"))
  (bind _asbp_shaft (cast `/Game/Workshop/Blueprints/BP_Shaft` OtherActor))
  (`/Engine/EditorBlueprintResources/StandardMacros.IsValid` _asbp_shaft
    (:`Is Valid`
      (`KismetSystemLibrary.PrintString` "overlap"))))

(event `self.StaticMeshComponent.OnComponentEndOverlap`
  (params (OverlappedComponent :type "PrimitiveComponent Object Reference") (OtherActor :type "Actor Object Reference") (OtherComp :type "PrimitiveComponent Object Reference") (OtherBodyIndex :type Integer))
  (bind _asbp_shaft (cast `/Game/Workshop/Blueprints/BP_Shaft` OtherActor))
  (`/Engine/EditorBlueprintResources/StandardMacros.IsValid` _asbp_shaft
    (:`Is Valid`
      (`KismetSystemLibrary.PrintString` "end overlap"))))

(event `self.StaticMeshComponent.OnComponentHit`
  (params (HitComponent :type "PrimitiveComponent Object Reference") (OtherActor :type "Actor Object Reference") (OtherComp :type "PrimitiveComponent Object Reference") (NormalImpulse :type "Vector Structure") (Hit :type "HitResult Structure (by ref)"))
  (bind _output_get (set `self.bOnTable` (`self.ActorHasTag` OtherActor "Table")))
  (if _output_get
    (`self.OnLandedOnTable`)
    (clear `self.OnLandedOnTable`)
    (elif (`self.ActorHasTag` OtherActor "Ground")
      (`self.OnLandedOnGround`)
      (`GameplayStatics.PlaySound2D` "/Game/Workshop/Audio/metal-cup-drop-105939.metal-cup-drop-105939" 1.0 1.0 0.0 null null))))

(fn `Rotate`
  (params (Rotation :type "Rotator Structure"))
  (`SceneComponent.K2_AddRelativeRotation` (`self.Inner_racing__Inner_racing_48`) Rotation false false))

(fn `UserConstructionScript`)