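; BP_Shaft is a workshop shaft that accepts parts the player drops onto it.
; Overlap binds to the part's GrabbableTool drop event; leaving unbinds it and resets its grab type to free.
; SnapObject attaches parts tagged "New" to the Head socket, then a Timeline slides them to Bearing1 and calls OnPlacedOnShaft.
; Untagged parts play an error sound and return to their stored transform.
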(event `self.ReceiveActorBeginOverlap`
  (params (OtherActor :type "Actor Object Reference"))
  (bind _returnvalue (`self.GetComponentByClass` OtherActor "/Game/Workshop/Blueprints/GrabbableTool.GrabbableTool_C"))
  (`/Engine/EditorBlueprintResources/StandardMacros.IsValid` _returnvalue
    (:`Is Valid`
      (set `self.Other Actor` OtherActor)
      (add `/Game/VRTemplate/Blueprints/GrabComponent.OnDropped` _returnvalue (`|CreateDelegate` :!event `SnapObject`)))))

(event `self.ReceiveActorEndOverlap`
  (params (OtherActor :type "Actor Object Reference"))
  (bind _returnvalue (`self.GetComponentByClass` OtherActor "/Game/Workshop/Blueprints/GrabbableTool.GrabbableTool_C"))
  (`/Engine/EditorBlueprintResources/StandardMacros.IsValid` _returnvalue
    (:`Is Valid`
      (clear `/Game/VRTemplate/Blueprints/GrabComponent.OnDropped` _returnvalue)
      ;[1 1 1] set grabtype to free so overlapped component can be attached to controller
      (set `/Game/VRTemplate/Blueprints/GrabComponent.GrabType` "NewEnumerator4" _returnvalue))))

(event `SnapObject`
  (bind _other_actor (`self.Other Actor`))
  (bind _staticmeshcomponent (`self.StaticMeshComponent`))
  (bind _other_actor_2 (`self.Other Actor`))
  (bind _returnvalue (`self.GetComponentByClass` (`self.Other Actor`) "/Game/Workshop/Blueprints/GrabbableTool.GrabbableTool_C"))
  (if (`self.ActorHasTag` _other_actor "New")
    (`PrimitiveComponent.SetSimulatePhysics` (`self.GetComponentByClass` _other_actor "/Script/Engine.StaticMeshComponent") false)
    (bind _returnvalue_2 (`self.K2_AttachToComponent` _other_actor_2 (`self.StaticMeshComponent`) "Head" "SnapToTarget" "SnapToTarget" "SnapToTarget" false))
    (if _returnvalue_2
      (`GameplayStatics.PlaySound2D` "/Game/Workshop/PUMP/correct-6033.correct-6033" 1.0 1.0 0.0 null null)
      (bind (_direction _newtrack_0) (`Timeline|Timeline`)
        (:`Update`
          (`self.K2_SetActorLocation` _other_actor_2 (`KismetMathLibrary.VLerp` (`SceneComponent.GetSocketLocation` _staticmeshcomponent "Head") (`SceneComponent.GetSocketLocation` _staticmeshcomponent "Bearing1") _newtrack_0) false false))
        (:`Finished`
          (`self.OnPlacedOnShaft`))))
    (else
      (`GameplayStatics.PlaySound2D` "/Game/Workshop/Audio/wrong-47985.wrong-47985" 2.0 1.0 0.0 null null)
      (`SceneComponent.K2_SetWorldTransform` (`SceneComponent.GetAttachParent` _returnvalue) (`/Game/Workshop/Blueprints/GrabbableTool.OldLocation` _returnvalue) false false))))

(fn `UserConstructionScript`)